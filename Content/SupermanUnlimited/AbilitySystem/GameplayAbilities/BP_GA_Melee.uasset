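; BP_GA_Melee is a gameplay ability for a melee attack, currently only a debug hit probe.
; On activation it sphere-traces on the Visibility channel along the owner actor's forward vector, starting just ahead of its location, with timed debug drawing.
; It prints whether the trace hit and ends immediately, applying no damage, effects or animation.
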(event `self.K2_ActivateAbility`
  (bind _owneractor (break `GameplayAbilityActorInfo` (`self.GetActorInfo`)))
  (bind _returnvalue (`Actor.K2_GetActorLocation` _owneractor))
  (bind _returnvalue_2 (`Actor.GetActorForwardVector` _owneractor))
  (bind (_outhit _returnvalue_3) (`KismetSystemLibrary.SphereTraceSingle` :`Start` (+ _returnvalue (* _returnvalue_2 50.0)) :`End` (+ _returnvalue (* _returnvalue_2 500.0)) :`Radius` 50.0 :`TraceChannel` "TraceTypeQuery1" :`DrawDebugType` "ForDuration"))
  (`KismetSystemLibrary.PrintString` (`KismetStringLibrary.Conv_BoolToString` _returnvalue_3))
  (`self.K2_EndAbility`))